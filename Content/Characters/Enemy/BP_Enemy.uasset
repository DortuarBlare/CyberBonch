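; Enemy character Blueprint that handles melee attacks on the player, taking damage and death.
; Player overlap with AttackSphere sets the attacking flag, while ApplyDamage rechecks the overlap before damaging BP_Player.
; TakeDamage lowers Health, jumps the animation state machine to death or, after a short delay, a hit reaction, and disables movement in both cases without re-enabling it here.
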(event OnComponentBeginOverlap(AttackSphere)
  (params (OverlappedComponent :type Primitive%20Component%20Object%20Reference) (OtherActor :type Actor%20Object%20Reference) (OtherComp :type Primitive%20Component%20Object%20Reference) (OtherBodyIndex :type Integer) (bFromSweep :type Boolean) (SweepResult :type Hit%20Result%20Structure%20%28by%20ref%29))
  (Utilities|Casting|CastToBP_Player OtherActor)
  (Variables|Default|SetIsAttacking true))

(event Custom|TakeDamage
  (params (DamagePoints :type Float%20%28double-precision%29))
  (bind _animationcomponent (Variables|Default|GetAnimationComponent))
  (bind _animinstance (Variables|/Script/PaperZD.PaperZDAnimationComponent|GetAnimInstance _animationcomponent))
  (bind _output_get (Variables|Default|SetHealth (- (Variables|Default|GetHealth) DamagePoints)))
  (if (and (<= _output_get 0.0) (not (Variables|Default|GetIsDead)))
    (Variables|Default|SetIsDead true)
    (Class|PaperZDAnimInstance|JumptoNode _animinstance "ToDeath" "None")
    (else
      (Variables|Default|SetIsTakingDamage true)
      (Utilities|FlowControl|Delay 0.1)
      (Class|PaperZDAnimInstance|JumptoNode _animinstance "ToTakingDamage" "None")
      (Development|PrintString "Enemy taking damage")))
  (Pawn|Components|CharacterMovement|DisableMovement (Variables|Character|GetCharacterMovement)))

(event Custom|ApplyDamage
  (CallFunction|CheckAttackSphere))

(fn ConstructionScript)

(fn CheckAttackSphere
  (bind _returnvalue (Game|GetPlayerCharacter 0))
  (if (Collision|IsOverlappingActor (Variables|Default|GetAttackSphere) _returnvalue :!class /Script/Engine.PrimitiveComponent)
    (bind _asbp_player (Utilities|Casting|CastToBP_Player _returnvalue))
    (Default|TakeDamage _asbp_player (Variables|Default|GetDamagePoints))))