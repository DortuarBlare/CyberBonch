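; BP_SpikePlatforms is a trap platform whose spikes rise when the player steps on it and damage the player on contact.
; Overlapping BoxEarth raises BoxSpark after a short delay, then lowers it again, with a flag blocking retriggers during the cycle.
; Overlapping BoxSpark damages the player through their HealthComponent, with a second flag and delay acting as a brief hit cooldown.
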(event OnComponentBeginOverlap(BoxSpark)
  (params (OverlappedComponent :type Primitive%20Component%20Object%20Reference) (OtherActor :type Actor%20Object%20Reference) (OtherComp :type Primitive%20Component%20Object%20Reference) (OtherBodyIndex :type Integer) (bFromSweep :type Boolean) (SweepResult :type Hit%20Result%20Structure%20%28by%20ref%29))
  (bind _asbp_player (Utilities|Casting|CastToBP_Player OtherActor))
  (if (and (Variables|Default|GetisOverlap) (stale _bsuccess))
    (Variables|Default|SetisOverlap false)
    (Default|TakeDamage (Variables|/Game/Characters/Player/BP_Player.BP_Player_C|GetHealth%20Component _asbp_player) 1.0)
    (Utilities|FlowControl|Delay 0.5)
    (Variables|Default|SetisOverlap true)))

(event OnComponentBeginOverlap(BoxEarth)
  (params (OverlappedComponent :type Primitive%20Component%20Object%20Reference) (OtherActor :type Actor%20Object%20Reference) (OtherComp :type Primitive%20Component%20Object%20Reference) (OtherBodyIndex :type Integer) (bFromSweep :type Boolean) (SweepResult :type Hit%20Result%20Structure%20%28by%20ref%29))
  (bind _boxspark (Variables|Default|GetBoxSpark))
  (if (and (.bSuccess (Utilities|Casting|CastToBP_Player OtherActor)) (Variables|Default|GetisSpark))
    (Variables|Default|SetisSpark false)
    (Utilities|FlowControl|Delay 0.5)
    (Transformation|AddRelativeLocation _boxspark "0, 0,60.000000" false false)
    (Utilities|FlowControl|Delay 1.5)
    (Transformation|AddRelativeLocation _boxspark "0, 0,-60.000000" false false)
    (Variables|Default|SetisSpark true)))

(fn ConstructionScript)